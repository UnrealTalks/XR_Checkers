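; Board actor that builds a checkered grid of squares, sized by BoardSize and SquareSize.
; The construction script gets tile positions and colours from TileLocations, then adds scaled instances to the DarkSquares or LightSquares component.
; On BeginPlay it sends its dimensions and transform to the game mode through PopulateBoardMessage and prints a debug string.
; An unconnected nested-loop version of the grid layout remains in the construction script.
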(event `self.ReceiveBeginPlay`
  (message `/Game/Blueprints/BoardInterface.PopulateBoard` (`GameplayStatics.GetGameMode`) (`self.SquareSize`) (`self.BoardSize`) (`self.GetTransform`))
  (`KismetSystemLibrary.PrintString` "event called" true false))

(fn `UserConstructionScript`
  (bind _squaresize (`self.SquareSize`))
  (bind _locations (`/Game/Blueprints/BoardFunctions.TileLocations` (`self.SquareSize`) (`self.BoardSize`)))
  (for _array_element _locations
    (if (`.Dark?_5_2536DA5A4BC1867FF1DD0B99A4FED55D` (break `/Game/Blueprints/TileStruct` _array_element))
      (`InstancedStaticMeshComponent.AddInstance` (`self.DarkSquares`) (`KismetMathLibrary.MakeTransform` (break `/Game/Blueprints/TileStruct` _array_element) (struct) (`KismetMathLibrary.MakeVector` _squaresize _squaresize 1.0)))
      (else
        (`InstancedStaticMeshComponent.AddInstance` (`self.LightSquares`) (`KismetMathLibrary.MakeTransform` (break `/Game/Blueprints/TileStruct` _array_element) (struct) (`KismetMathLibrary.MakeVector` _squaresize _squaresize 1.0)))))))