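; BoardFunctions holds helper functions that compute tile and starting piece positions for a checkers-style board.
; TileLocations builds a square grid of tile centers around the origin at zero height, flagging tiles dark by index parity.
; PieceLocations takes that array, derives the board width from the square root of its length, and collects dark tiles from the first or last rows depending on the player.
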(fn `PieceLocations`
  (params (TileLocations :type "Array of /Game/Blueprints/TileStruct Structure") (`PlayerOne?` :type Boolean) (NumOfRows :type Integer))
  (returns (PieceLocations :type "Array of Vector Structure"))
  (locals (Locations_ :type "Array of Vector Structure"))
  (bind _returnvalue (`KismetArrayLibrary.Array_Length` TileLocations))
  (bind _returnvalue_2 (* NumOfRows (`KismetMathLibrary.FTrunc` (`KismetMathLibrary.Sqrt` (`KismetMathLibrary.Conv_IntToDouble` _returnvalue)))))
  (`|ExecutionSequence`
    (:`then_0`
      (if `PlayerOne?`
        (for _index (range (+ _returnvalue_2 1))
          (bind (_output_location _output_dark_) (break `/Game/Blueprints/TileStruct` (`|GetArrayItem` (`local.TileLocations`) _index)))
          (if _output_dark_
            (`KismetArrayLibrary.Array_Add` (`local.Locations_`) _output_location)))
        (else
          (for _index_2 (range (- _returnvalue _returnvalue_2) (+ _returnvalue 1))
            (bind (_output_location_2 _output_dark__2) (break `/Game/Blueprints/TileStruct` (`|GetArrayItem` (`local.TileLocations`) _index_2)))
            (if _output_dark__2
              (`KismetArrayLibrary.Array_Add` (`local.Locations_`) _output_location_2))))))
    (:`then_1`
      (return (`local.Locations_`)))))

(fn `TileLocations`
  (params (SquareSize :type "Float (double-precision)") (BoardSize :type Integer))
  (returns (Locations :type "Array of /Game/Blueprints/TileStruct Structure"))
  (locals (Locations_ :type "Array of /Game/Blueprints/TileStruct Structure"))
  (bind _returnvalue (- BoardSize 1))
  (bind _squaresize (`local.SquareSize`))
  (bind _returnvalue_2 (/ _squaresize 2.0))
  (bind _returnvalue_3 (* (/ (`KismetMathLibrary.Conv_IntToDouble` BoardSize) -2.0) (`local.SquareSize`)))
  (`|ExecutionSequence`
    (:`then_0`
      (for _index (range (+ _returnvalue 1))
        (for _index_2 (range (+ _returnvalue 1))
          (`KismetArrayLibrary.Array_Add` (`local.Locations_`) (make `/Game/Blueprints/TileStruct` (`KismetMathLibrary.MakeVector` (+ (* _index _squaresize) _returnvalue_3 _returnvalue_2) (+ (* _index_2 (`local.SquareSize`)) _returnvalue_3 _returnvalue_2)) (== (mod (+ _index _index_2) 2) 0))))))
    (:`then_1`
      (return (`local.Locations_`)))))