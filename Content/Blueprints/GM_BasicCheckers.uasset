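; Basic checkers game mode that fills the board with starting pieces for both players.
; PopulateBoard computes tile locations from the square and board size, then derives three starting rows for each side.
; It spawns a BP_Checker at each location, offset from the world transform and slightly raised, scaled to the square size and flagged by player.
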(event `/Game/Blueprints/BoardInterface.PopulateBoard`
  (params (SquareSize :type "Float (single-precision)") (BoardSize :type Integer) (WorldTransform :type "Transform Structure"))
  (bind _returnvalue (`KismetMathLibrary.Conv_DoubleToVector` (/ SquareSize 12.0)))
  (bind _locations (`/Game/Blueprints/BoardFunctions.TileLocations` SquareSize BoardSize))
  (`|ExecutionSequence`
    (:`then_0`
      (bind _piecelocations (`/Game/Blueprints/BoardFunctions.PieceLocations` _locations true 3))
      (for _array_element _piecelocations
        (`|SpawnActorFromClass` "/Game/Blueprints/BP_Checker.BP_Checker_C" (`KismetMathLibrary.MakeTransform` (+ WorldTransform_Location _array_element (0.0 0.0 0.5)) (struct) _returnvalue) "Undefined" "OverrideRootScale" null true null)))
    (:`then_1`
      (bind _piecelocations_2 (`/Game/Blueprints/BoardFunctions.PieceLocations` _locations false 3))
      (for _array_element_2 _piecelocations_2
        (`|SpawnActorFromClass` "/Game/Blueprints/BP_Checker.BP_Checker_C" (`KismetMathLibrary.MakeTransform` (+ WorldTransform_Location _array_element_2 (0.0 0.0 0.5)) (struct) _returnvalue) "Undefined" "OverrideRootScale" null false null)))))

(fn `UserConstructionScript`)